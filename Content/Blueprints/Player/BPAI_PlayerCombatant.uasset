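; Player combatant Blueprint that gives visual feedback for taking damage and attacking, and unhides itself shortly after BeginPlay.
; HealthComp damage events swap to a damaged sprite material and back around a backward nudge, though the SetMaterial function itself is empty here.
; CombatData attack events trigger a forward nudge through the same NudgeCharacter event.
; Two chained timelines lerp the actor along its forward vector and back.
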(event OnTakeDamage(HealthComp)
  ;[0.15 0.15 0.15 0.5] Flashes the damage material for a second and then returns it back to its original
  (Development|PrintString "Player On Damage Called")
  (Utilities|FlowControl|Delay 0.1)
  (CallFunction|SetMaterial "/Game/Materials/TestSprite_DamagedMat.TestSprite_DamagedMat")
  (CallFunction|NudgeCharacter -3e+01)
  (Utilities|FlowControl|Delay 0.2)
  (CallFunction|SetMaterial "/Paper2D/MaskedLitSpriteMaterial.MaskedLitSpriteMaterial"))

(event OnAttackCommence(CombatData)
  (params (AttackType :type EAttackType%20Enum :default "Close") (HitSuccessful :type Boolean))
  (CallFunction|NudgeCharacter 3e+01))

(event Custom|NudgeCharacter
  (params (Desired%20Offset :type Float%20%28double-precision%29))
  (bind (_current _target) (CallFunction|GetPointonActorX Desired%20Offset))
  ;[0.15 0.15 0.15 0.5] Functionality for knockback, lerps the location back a bit then lerps it back forward to where it was.
  (Variables|Default|SetNudge_Current _current)
  (Variables|Default|SetNudge_Target _target)
  (bind _alpha (Timeline|Timeline PlayFromStart)
    (:Update
      (Class|HealthComponent|LerpActorLocation (Variables|Default|GetHealthComp) self (Variables|Default|GetNudge_Current) (Variables|Default|GetNudge_Target) _alpha))
    (:Finished
      (bind _alpha_2 (Timeline|Timeline_0 PlayFromStart)
        (:Update
          (Class|HealthComponent|LerpActorLocation (Variables|Default|GetHealthComp) self (Variables|Default|GetNudge_Target) (Variables|Default|GetNudge_Current) _alpha_2))))))

(event EventBeginPlay
  (Utilities|FlowControl|Delay 0.05)
  (Rendering|SetActorHiddenInGame false))

(fn ConstructionScript)

(fn SetMaterial
  (params (Material :type Material%20Interface%20Object%20Reference)))

(fn GetPointonActorX
  (params (Offset :type Float%20%28double-precision%29))
  (return (Transformation|GetActorLocation) (+ (Transformation|GetActorLocation) (* (Transformation|GetActorForwardVector) Offset))))