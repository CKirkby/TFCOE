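; TestBPAI is a test AI Blueprint with a sprite and a health component that shows a hit flash when damaged.
; It deals one point of damage to itself shortly after BeginPlay.
; The damage event briefly swaps the sprite to a damaged material, then sets it to the masked lit sprite material.
; Each swap creates a new dynamic material instance.
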(event OnTakeDamage(HealthComp)
  ;[0.15 0.15 0.15 0.5] Flashes the damage material for a second and then returns it back to its original
  (CallFunction|SetMaterial "/Game/Materials/TestSprite_DamagedMat.TestSprite_DamagedMat")
  (Utilities|FlowControl|Delay 0.2)
  (CallFunction|SetMaterial "/Paper2D/MaskedLitSpriteMaterial.MaskedLitSpriteMaterial"))

(event EventBeginPlay
  (Utilities|FlowControl|Delay 3.0)
  (Class|HealthComponent|TakeDamage (Variables|Default|GetHealthComp) 1))

(fn ConstructionScript)

(fn SetMaterial
  (params (Material :type Material%20Interface%20Object%20Reference))
  (bind _returnvalue (Rendering|Material|CreateDynamicMaterialInstance Material "None" "None" :!class /Script/Engine.KismetMaterialLibrary))
  (Rendering|Material|SetMaterial (Variables|Default|GetSprite) 0 _returnvalue))