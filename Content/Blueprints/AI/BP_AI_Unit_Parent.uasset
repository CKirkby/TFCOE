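; Parent Blueprint for sprite-based AI units in grid combat, providing hit and attack feedback plus debug text for health and faction.
; Taking damage briefly swaps the sprite to a damage material instance, refreshes health text and nudges the unit backward.
; Close combat attacks nudge it forward.
; Nudges lerp out and back via two chained timelines, then a failsafe snaps any displaced unit to its CombatData grid position.
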(event OnTakeDamage(HealthComp)
  ;[0.15 0.15 0.15 0.5] Flashes the damage material for a second and then returns it back to its original
  (Utilities|FlowControl|Delay 0.1)
  (CallFunction|SetMaterial true)
  (Utilities|TESTUpdateHealthDebug
    (:Out
      (CallFunction|NudgeCharacter -3e+01)
      (Utilities|FlowControl|Delay 0.2)
      (CallFunction|SetMaterial false))))

(event OnAttackCommence(CombatData)
  (params (AttackType :type EAttackType%20Enum :default "Close") (HitSuccessful :type Boolean))
  ;[0.15 0.15 0.15 0.5] On Attack Functionality
  (switch Utilities|FlowControl|Switch|SwitchonEAttackType AttackType
    (:Close
      (CallFunction|NudgeCharacter 3e+01))))

(event Custom|NudgeCharacter
  (params (Desired%20Offset :type Float%20%28double-precision%29))
  (bind (_returnvalue _returnvalue2) (CallFunction|GetPointonActorX Desired%20Offset))
  ;[0.15 0.15 0.15 0.5] Functionality for knockback, lerps the location back a bit then lerps it back forward to where it was.
  (Variables|Default|SetNudge_Current _returnvalue)
  (Variables|Default|SetNudge_Target _returnvalue2)
  (bind _alpha (Timeline|SetNudge PlayFromStart)
    (:Update
      (Class|HealthComponent|LerpActorLocation (Variables|Default|GetHealthComp) self (Variables|Default|GetNudge_Current) (Variables|Default|GetNudge_Target) _alpha))
    (:Finished
      (bind _alpha_2 (Timeline|ReturnNudge PlayFromStart)
        (:Update
          (Class|HealthComponent|LerpActorLocation (Variables|Default|GetHealthComp) self (Variables|Default|GetNudge_Target) (Variables|Default|GetNudge_Current) _alpha_2))
        (:Finished
          (CallFunction|NudgeFailsafePosCheck))))))

(event EventBeginPlay
  (CallFunction|CreateDynamicMaterials))

(fn ConstructionScript
  (bind _combatdata (Variables|Default|GetCombatData))
  (bind _returnvalue (Class|CharacterCombatData|GetUnitConfiguration _combatdata))
  (Utilities|FlowControl|Sequence
    (:then_0
      (Utilities|IsValid _returnvalue
        (:Is%20Valid
          (Rendering|Components|TextRender|SetText (Variables|Default|GetID_Text) (Utilities|Text|ToText(String) (Utilities|String|Append (Utilities|String|EnumtoString (Variables|/Script/UntoParadise.UnitConfiguration|GetFactionID _returnvalue)) ": " (Utilities|String|EnumtoString (Variables|/Script/UntoParadise.UnitConfiguration|GetFactionRank _returnvalue))))))))
    (:then_1
      (Utilities|IsValid (Variables|Default|GetHealthComp)
        (:Is%20Valid
          (Utilities|TESTUpdateHealthDebug))))))

(fn SetMaterial
  (params (Damaged :type Boolean))
  (bind _sprite (Variables|Default|GetSprite))
  (if Damaged
    (Rendering|Material|SetMaterial _sprite 0 (Variables|Default|GetDamagedMat))
    (else
      (Rendering|Material|SetMaterial _sprite 0 (Variables|Default|GetNormalMat)))))

(fn GetPointonActorX
  (params (Desired%20Offset :type Float%20%28double-precision%29))
  (return (Transformation|GetActorLocation) (+ (Transformation|GetActorLocation) (* (Transformation|GetActorForwardVector) Desired%20Offset))))

(fn CreateDynamicMaterials
  (Utilities|FlowControl|Sequence
    (:then_0
      (bind _returnvalue (Rendering|Material|CreateDynamicMaterialInstance "/Game/Materials/TestSprite_DamagedMat.TestSprite_DamagedMat" "None" "None" :!class /Script/Engine.KismetMaterialLibrary))
      (Variables|Default|SetDamagedMat _returnvalue))
    (:then_1
      (bind _returnvalue_2 (Rendering|Material|CreateDynamicMaterialInstance "/Paper2D/MaskedLitSpriteMaterial.MaskedLitSpriteMaterial" "None" "None" :!class /Script/Engine.KismetMaterialLibrary))
      (Variables|Default|SetNormalMat _returnvalue_2))))

(fn NudgeFailsafePosCheck
  (bind _combatdata (Variables|Default|GetCombatData)
    (:then
      (if (Utilities|Operators|NotEqual(!=) (Transformation|GetActorLocation) (Variables|Default|GetNudge_Current) 0.0)
        (Transformation|SetActorLocation (Class|CharacterCombatData|GetGridPosition _combatdata (Class|CharacterCombatData|GetCurrentGridCoordinates _combatdata)) false false)))
    (:else)))