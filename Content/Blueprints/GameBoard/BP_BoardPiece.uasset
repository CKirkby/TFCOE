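; BP_BoardPiece is a game board piece with a box collider and a text label showing its grid coordinates or blocked state.
; The construction script checks CurrentPieceState: enabled pieces register the box collider and display their X,Y grid position, while disabled pieces display "Blocked".
; Box begin and end overlap events pass the other actor to TriggerOverlapFunctionality and TriggerOverlapEndFunctionality, which are defined outside these graphs.
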(event OnComponentBeginOverlap(BoxCollision)
  (params (OverlappedComponent :type Primitive%20Component%20Object%20Reference) (OtherActor :type Actor%20Object%20Reference) (OtherComp :type Primitive%20Component%20Object%20Reference) (OtherBodyIndex :type Integer) (bFromSweep :type Boolean) (SweepResult :type Hit%20Result%20Structure%20%28by%20ref%29))
  (Class|BoardPiece|TriggerOverlapFunctionality OtherActor))

(event OnComponentEndOverlap(BoxCollision)
  (params (OverlappedComponent :type Primitive%20Component%20Object%20Reference) (OtherActor :type Actor%20Object%20Reference) (OtherComp :type Primitive%20Component%20Object%20Reference) (OtherBodyIndex :type Integer))
  (Class|BoardPiece|TriggerOverlapEndFunctionality OtherActor))

(fn ConstructionScript
  (bind _returnvalue (Class|BoardPiece|GetGridPosition))
  (switch Utilities|FlowControl|Switch|SwitchonEPieceState (Variables|Default|GetCurrentPieceState)
    (:Enabled
      (Class|BoardPiece|SetBoxCollider (Variables|Default|GetBoxCollision))
      (Rendering|Components|TextRender|SetText (Variables|Default|GetTextRender) (Utilities|Text|ToText(String) (Utilities|String|Append (Utilities|String|ToString(Integer) (.x _returnvalue)) ", " (Utilities|String|ToString(Integer) (.y _returnvalue))))))
    (:Disabled
      (Rendering|Components|TextRender|SetText (Variables|Default|GetTextRender) (Utilities|Text|MakeLiteralText "Blocked")))))